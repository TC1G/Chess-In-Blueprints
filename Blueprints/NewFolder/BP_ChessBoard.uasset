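; Chess board actor that spawns both sides' pieces and runs turns, castling and check highlighting.
; Tiles are tagged mesh components whose names give the square keys for the AllPieces map.
; Selected pieces get highlight actors on valid tiles, and clicking a valid tile moves the piece.
; Moves by the current team refresh all pieces' moves, test for a missing king (GameOver is empty), toggle the player and highlight a checked king.
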(event Custom|PieceMoved
  (params (Team :type TeamEnum%20Enum :default "NewEnumerator0"))
  (if (Utilities|Enum|Equal(Enum) Team (CallFunction|GetCurentTeam))
    (CallFunction|EndTurn)))

(event Custom|Mouse%20Clicked
  (Variables|Default|SetCurrentPiece 0)
  (CallFunction|ClearHighlights))

(event Custom|PlayerClickedTiles
  (params (TouchedComponent :type Primitive%20Component%20Object%20Reference) (ButtonPressed :type Key%20Structure :default "None"))
  (CallFunction|MovetoTile TouchedComponent))

(event EventBeginPlay
  ;[1 1 1] Player Refference
  (bind _outactors (Actor|GetAllActorsOfClass "/Game/Blueprints/NewFolder/ChessCharacter.ChessCharacter_C"))
  (Variables|Default|SetPlayer%20Ref (Utilities|Array|Get(acopy) _outactors))
  (CallFunction|InitPieces)
  (Utilities|FlowControl|Delay 0.2)
  (bind _values (Utilities|Map|Values (Variables|Default|GetAll%20Pieces%20)))
  (CallFunction|UpdateMoves _values)
  (for _array_element _values
    (EventDispatchers|BindEventtoPieceMoved _array_element (delegate Custom|PieceMoved)))
  (bind _aschess_pc (Utilities|Casting|CastToChessPC (Game|GetPlayerController 0)))
  (EventDispatchers|AssignMouseClicked _aschess_pc (delegate Custom|Mouse%20Clicked))
  (for _array_element_2 (Actor|GetComponentsbyTag "/Script/Engine.StaticMeshComponent" "Tiles")
    (EventDispatchers|BindEventtoOnClicked _array_element_2 (delegate Custom|PlayerClickedTiles))))

(fn ConstructionScript)

(fn FindTileLetter
  (params (Tile :type Object%20Object%20Reference))
  (return (Utilities|String|LeftChop (Utilities|String|RightChop (Utilities|GetObjectName Tile) 6) 1)))

(fn FindTileNumber
  (params (Tile :type Object%20Object%20Reference))
  (return (Utilities|String|RightChop (Utilities|GetObjectName Tile) 7)))

(fn FindTileNumberandLetter
  (params (Tile :type Object%20Object%20Reference))
  (return (Utilities|String|RightChop (Utilities|GetObjectName Tile) 6)))

(fn SpawnPiece
  (params (Class :type BP%20Piece%20Parent%20Class%20Reference) (Team :type TeamEnum%20Enum :default "NewEnumerator0") (Tile :type Static%20Mesh%20Component%20Object%20Reference))
  (bind _number (CallFunction|FindTileNumberandLetter Tile))
  (bind _returnvalue (Game|SpawnActorfromClass Class (Math|Transform|MakeTransform (Transformation|GetWorldLocation Tile) (Utilities|Select :Index Team :NewEnumerator0 "0, 0, 0" :NewEnumerator1 "0.000000,180.000000,0.000000")) "Undefined" 0 0))
  (Utilities|Map|Add (Variables|Default|GetAll%20Pieces%20) _number _returnvalue)
  (Default|Init _returnvalue Team _number self)
  (return _returnvalue))

(fn InitPieces
  (Utilities|FlowControl|Sequence
    (:then_0
      (for _array_element (Actor|GetComponentsbyTag "/Script/Engine.StaticMeshComponent" "Tiles")
        (if (Utilities|Enum|Equal(Enum) (CallFunction|FindTileLetter _array_element) "B")
          (CallFunction|SpawnPiece "/Game/Blueprints/NewFolder/Pieces/BP_Pawn.BP_Pawn_C" "NewEnumerator0" _array_element)
          (elif (Utilities|Enum|Equal(Enum) (CallFunction|FindTileLetter _array_element) "G")
            (CallFunction|SpawnPiece "/Game/Blueprints/NewFolder/Pieces/BP_Pawn.BP_Pawn_C" "NewEnumerator1" _array_element)))))
    (:then_1
      (for _array_element_2 (Utilities|Array|MakeArray (Variables|Default|GetBlock_H1) (Variables|Default|GetBlock_H8))
        (CallFunction|SpawnPiece "/Game/Blueprints/NewFolder/Pieces/BP_Rook.BP_Rook_C" "NewEnumerator1" _array_element_2))
      (for _array_element_3 (Utilities|Array|MakeArray (Variables|Default|GetBlock_A1) (Variables|Default|GetBlock_A8))
        (CallFunction|SpawnPiece "/Game/Blueprints/NewFolder/Pieces/BP_Rook.BP_Rook_C" "NewEnumerator0" _array_element_3)))
    (:then_2
      (for _array_element_4 (Utilities|Array|MakeArray (Variables|Default|GetBlock_H7) (Variables|Default|GetBlock_H2))
        (CallFunction|SpawnPiece "/Game/Blueprints/NewFolder/Pieces/BP_Knight.BP_Knight_C" "NewEnumerator1" _array_element_4))
      (for _array_element_5 (Utilities|Array|MakeArray (Variables|Default|GetBlock_A7) (Variables|Default|GetBlock_A2))
        (CallFunction|SpawnPiece "/Game/Blueprints/NewFolder/Pieces/BP_Knight.BP_Knight_C" "NewEnumerator0" _array_element_5)))
    (:then_3
      (for _array_element_6 (Utilities|Array|MakeArray (Variables|Default|GetBlock_H6) (Variables|Default|GetBlock_H3))
        (CallFunction|SpawnPiece "/Game/Blueprints/NewFolder/Pieces/BP_Bishop.BP_Bishop_C" "NewEnumerator1" _array_element_6))
      (for _array_element_7 (Utilities|Array|MakeArray (Variables|Default|GetBlock_A3) (Variables|Default|GetBlock_A6))
        (CallFunction|SpawnPiece "/Game/Blueprints/NewFolder/Pieces/BP_Bishop.BP_Bishop_C" "NewEnumerator0" _array_element_7)))
    (:then_4
      (CallFunction|SpawnPiece "/Game/Blueprints/NewFolder/Pieces/BP_Queen.BP_Queen_C" "NewEnumerator0" (Variables|Default|GetBlock_A5))
      (CallFunction|SpawnPiece "/Game/Blueprints/NewFolder/Pieces/BP_Queen.BP_Queen_C" "NewEnumerator1" (Variables|Default|GetBlock_H5)))
    (:then_5
      (bind _piece_reference (CallFunction|SpawnPiece "/Game/Blueprints/NewFolder/Pieces/BP_King.BP_King_C" "NewEnumerator0" (Variables|Default|GetBlock_A4)))
      (Variables|Default|SetWhite%20King _piece_reference)
      (bind _piece_reference_2 (CallFunction|SpawnPiece "/Game/Blueprints/NewFolder/Pieces/BP_King.BP_King_C" "NewEnumerator1" (Variables|Default|GetBlock_H4)))
      (Variables|Default|SetBlack%20King _piece_reference_2))))

(fn GetCurentTeam
  (return (Variables|/Game/Blueprints/NewFolder/ChessCharacter.ChessCharacter_C|GetTeam (Variables|Default|GetPlayer%20Ref))))

(fn GetPositionInfo
  (params (Position :type String))
  (bind _all_pieces_ (Variables|Default|GetAll%20Pieces%20))
  (bind (_value _returnvalue) (Utilities|Map|Find _all_pieces_ Position))
  (if _returnvalue
    (Utilities|IsValid _value
      (:Is%20Valid
        (return _value true (Variables|/Game/Blueprints/NewFolder/Pieces/BP_Piece_Parent.BP_Piece_Parent_C|GetTeam _value))))
    (else
      (return 0 false "NewEnumerator0"))))

(fn UpdateMoves
  (params (Array :type Array%20of%20BP%20Piece%20Parent%20Object%20References))
  (for _array_element Array
    (Default|RefreshMoves _array_element)))

(fn HighlightValidPoints
  (params (Positions :type Array%20of%20Strings))
  (for _array_element (Actor|GetComponentsbyTag "/Script/Engine.StaticMeshComponent" "Tiles")
    (if (Utilities|Array|ContainsItem Positions (CallFunction|FindTileNumberandLetter _array_element))
      (bind _returnvalue (Game|SpawnActorfromClass "/Game/Blueprints/NewFolder/Highlights/BP_HighlightActor.BP_HighlightActor_C" (Math|Transform|MakeTransform (Math|Vector|MakeVector (.X (Math|Vector|BreakVector (Transformation|GetWorldLocation _array_element))) (.Y (Math|Vector|BreakVector (Transformation|GetWorldLocation _array_element))) (+ (.Z (Math|Vector|BreakVector (Transformation|GetWorldLocation _array_element))) 3.0))) "Undefined" 0 0))
      (Utilities|Array|Add (Variables|Default|GetHighlightActors) _returnvalue))))

(fn OnPieceSelected
  (params (CurrentPiece :type BP%20Piece%20Parent%20Object%20Reference) (Positions :type Array%20of%20Strings))
  (Variables|Default|SetCurrentPiece CurrentPiece)
  (CallFunction|HighlightValidPoints Positions))

(fn MovetoTile
  (params (Tile :type Primitive%20Component%20Object%20Reference))
  (bind _number (CallFunction|FindTileNumberandLetter Tile))
  (bind _currentpiece (Variables|Default|GetCurrentPiece))
  (Utilities|IsValid _currentpiece
    (:Is%20Valid
      (bind (_movement _attacks) (Default|GetAllPossibleMoves _currentpiece))
      (if (Utilities|Array|ContainsItem _movement _number)
        (CallFunction|Castle Tile :!label _label)
        (Default|MovePiece (Variables|Default|GetCurrentPiece) Tile)
        (elif (Utilities|Array|ContainsItem _attacks _number)
          (goto _label))))))

(fn EndTurn
  (bind _values (Utilities|Map|Values (Variables|Default|GetAll%20Pieces%20)))
  (CallFunction|UpdateMoves _values)
  (CallFunction|KingDeathCheck _values)
  (Default|TogglePlayer (Variables|Default|GetPlayer%20Ref))
  (CallFunction|ClearHighlightsKing)
  (if (CallFunction|IsKinginCheck)
    (CallFunction|HighlightCheckedKing)))

(fn ClearHighlights
  (for _array_element (Variables|Default|GetHighlightActors)
    (Utilities|IsValid _array_element
      (:Is%20Valid
        (Actor|DestroyActor _array_element)))))

(fn IsPositioninDanger
  (params (Position :type String) (Team :type TeamEnum%20Enum :default "NewEnumerator0"))
  (if (== (Utilities|String|Len Position) 2)
    (bind _values (Utilities|Map|Values (Variables|Default|GetAll%20Pieces%20)))
    (bind _array_element (Utilities|Array|ForEachLoopwithBreak _values :!label _label)
      (:LoopBody
        (if (Utilities|Enum|NotEqual(Enum) (Variables|/Game/Blueprints/NewFolder/Pieces/BP_Piece_Parent.BP_Piece_Parent_C|GetTeam _array_element) Team)
          (if (Utilities|Array|ContainsItem (Variables|/Game/Blueprints/NewFolder/Pieces/BP_Piece_Parent.BP_Piece_Parent_C|GetCurrent%20Movements _array_element) Position)
            (LocalVariables|SetReturn%20 true)
            (goto _label Break)
            (elif (Utilities|Array|ContainsItem (Variables|/Game/Blueprints/NewFolder/Pieces/BP_Piece_Parent.BP_Piece_Parent_C|GetCurrent%20Attacks _array_element) Position)
              (LocalVariables|SetReturn%20 true)
              (goto _label Break)))))
      (:Completed
        (return (LocalVariables|GetReturn%20))))))

(fn GetCurrentKing
  (return (Utilities|Select :Index (Variables|/Game/Blueprints/NewFolder/ChessCharacter.ChessCharacter_C|GetTeam (Variables|Default|GetPlayer%20Ref)) :NewEnumerator0 (Variables|Default|GetWhite%20King) :NewEnumerator1 (Variables|Default|GetBlack%20King))))

(fn IsKinginCheck
  (return (CallFunction|IsPositioninDanger (Variables|/Game/Blueprints/NewFolder/Pieces/BP_Piece_Parent.BP_Piece_Parent_C|GetPosition (CallFunction|GetCurrentKing)) (CallFunction|GetCurentTeam))))

(fn KingDeathCheck
  (params (Piece :type Array%20of%20BP%20Piece%20Parent%20Object%20References))
  (if (Utilities|Array|ContainsItem Piece (Variables|Default|GetBlack%20King))
    (if (not (Utilities|Array|ContainsItem Piece (Variables|Default|GetWhite%20King)))
      (CallFunction|GameOver))
    (else
      (CallFunction|GameOver))))

(fn GameOver)

(fn Castle
  (params (Block :type Object%20Object%20Reference))
  (bind _team (CallFunction|GetCurentTeam))
  (bind _number (CallFunction|FindTileNumberandLetter Block))
  (bind _team_2 (CallFunction|GetCurentTeam))
  (bind _asbp_king (Utilities|Casting|CastToBP_King (CallFunction|GetCurrentKing)))
  (if (Utilities|Map|Contains (Variables|/Game/Blueprints/NewFolder/Pieces/BP_King.BP_King_C|GetCastlinPoints _asbp_king) _number)
    (if (.ReturnValue (Utilities|Map|Find (Variables|Default|GetAll%20Pieces%20) (Utilities|Select :Index (.Value (Utilities|Map|Find (Variables|/Game/Blueprints/NewFolder/Pieces/BP_King.BP_King_C|GetCastlinPoints _asbp_king) _number)) :NewEnumerator0 (Utilities|Select :Index _team :NewEnumerator0 (Utilities|String|MakeLiteralString "A1") :NewEnumerator1 (Utilities|String|MakeLiteralString "H8")) :NewEnumerator1 (Utilities|Select :Index _team :NewEnumerator0 (Utilities|String|MakeLiteralString "A8") :NewEnumerator1 (Utilities|String|MakeLiteralString "H1")) :NewEnumerator2 "" :NewEnumerator3 "" :NewEnumerator4 "" :NewEnumerator5 "" :NewEnumerator6 "" :NewEnumerator7 "")))
      (if (not (Variables|/Game/Blueprints/NewFolder/Pieces/BP_Piece_Parent.BP_Piece_Parent_C|GetHasMoved (.Value (Utilities|Map|Find (Variables|Default|GetAll%20Pieces%20) (Utilities|Select :Index (.Value (Utilities|Map|Find (Variables|/Game/Blueprints/NewFolder/Pieces/BP_King.BP_King_C|GetCastlinPoints _asbp_king) _number)) :NewEnumerator0 (Utilities|Select :Index _team :NewEnumerator0 (Utilities|String|MakeLiteralString "A1") :NewEnumerator1 (Utilities|String|MakeLiteralString "H8")) :NewEnumerator1 (Utilities|Select :Index _team :NewEnumerator0 (Utilities|String|MakeLiteralString "A8") :NewEnumerator1 (Utilities|String|MakeLiteralString "H1")) :NewEnumerator2 "" :NewEnumerator3 "" :NewEnumerator4 "" :NewEnumerator5 "" :NewEnumerator6 "" :NewEnumerator7 "")))))
        (Default|MovePiece (.Value (Utilities|Map|Find (Variables|Default|GetAll%20Pieces%20) (Utilities|Select :Index (.Value (Utilities|Map|Find (Variables|/Game/Blueprints/NewFolder/Pieces/BP_King.BP_King_C|GetCastlinPoints _asbp_king) _number)) :NewEnumerator0 (Utilities|Select :Index _team :NewEnumerator0 (Utilities|String|MakeLiteralString "A1") :NewEnumerator1 (Utilities|String|MakeLiteralString "H8")) :NewEnumerator1 (Utilities|Select :Index _team :NewEnumerator0 (Utilities|String|MakeLiteralString "A8") :NewEnumerator1 (Utilities|String|MakeLiteralString "H1")) :NewEnumerator2 "" :NewEnumerator3 "" :NewEnumerator4 "" :NewEnumerator5 "" :NewEnumerator6 "" :NewEnumerator7 ""))) (Utilities|Select :Index (.Value (Utilities|Map|Find (Variables|/Game/Blueprints/NewFolder/Pieces/BP_King.BP_King_C|GetCastlinPoints _asbp_king) _number)) :NewEnumerator0 (Utilities|Select :Index _team_2 :NewEnumerator0 (Variables|Default|GetBlock_A3) :NewEnumerator1 (Variables|Default|GetBlock_H6)) :NewEnumerator1 (Utilities|Select :Index _team_2 :NewEnumerator0 (Variables|Default|GetBlock_A6) :NewEnumerator1 (Variables|Default|GetBlock_H3)) :NewEnumerator2 0 :NewEnumerator3 0 :NewEnumerator4 0 :NewEnumerator5 0 :NewEnumerator6 0 :NewEnumerator7 0))))))

(fn NewFunction)

(fn HighlightCheckedKing
  (for _array_element (Actor|GetComponentsbyTag "/Script/Engine.StaticMeshComponent" "Tiles")
    (if (Utilities|Enum|Equal(Enum) (CallFunction|FindTileNumberandLetter _array_element) (Variables|/Game/Blueprints/NewFolder/Pieces/BP_Piece_Parent.BP_Piece_Parent_C|GetPosition (CallFunction|GetCurrentKing)))
      (bind _returnvalue (Game|SpawnActorfromClass "/Game/Blueprints/NewFolder/Highlights/BP_KingCheck.BP_KingCheck_C" (Math|Transform|MakeTransform (Math|Vector|MakeVector (.X (Math|Vector|BreakVector (Transformation|GetWorldLocation _array_element))) (.Y (Math|Vector|BreakVector (Transformation|GetWorldLocation _array_element))) (+ (.Z (Math|Vector|BreakVector (Transformation|GetWorldLocation _array_element))) 3.0))) "Undefined" 0 0))
      (Utilities|Array|Add (Variables|Default|GetKingCheckHighlight) _returnvalue))))

(fn ClearHighlightsKing
  (for _array_element (Variables|Default|GetKingCheckHighlight)
    (Utilities|IsValid _array_element
      (:Is%20Valid
        (Actor|DestroyActor _array_element)))))