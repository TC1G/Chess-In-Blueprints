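; Pawn piece Blueprint for a chess-style board game that computes the piece's possible moves and attacks.
; GetAllPossibleMoves traces a path in one direction, two squares until the piece has moved and one afterward, keeping unoccupied squares as moves.
; It checks one square in each of two other directions for opposing-team pieces as attacks.
; Both checks query the board reference, and both result arrays are cleaned before return.
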(event EventBeginPlay
  (|CallParentFunction) ; This node is disabled and will not be called.\nDrag off pins to build functionality.
)

(fn ConstructionScript
  (|CallParentFunction))

(fn PawnAttackCheck
  (params (Position :type String))
  (bind _board_reference (Variables|Default|GetBoard%20Reference))
  (bind (_piece _piece_found _team) (Default|GetPositionInfo _board_reference Position))
  (return (and (== _piece_found true) (Utilities|Enum|NotEqual(Enum) _team (Variables|Default|GetTeam)))))

(fn PawnMovementCheck
  (params (Position :type String))
  (return (not (.Piece%20Found (Default|GetPositionInfo (Variables|Default|GetBoard%20Reference) Position)))))

(fn GetAllPossibleMoves
  (bind _local_array1 (CallFunction|FindValidPath (select (Variables|Default|GetHasMoved) 1 2) "NewEnumerator2"))
  (for _array_element _local_array1
    (if (CallFunction|PawnMovementCheck _array_element)
      (Utilities|Array|Add (LocalVariables|GetMovement%20Array) _array_element)))
  (for _array_element_2 (Utilities|Array|MakeArray "NewEnumerator3" "NewEnumerator4")
    (bind _local_array1_2 (CallFunction|FindValidPath 1 _array_element_2))
    (for _array_element_3 _local_array1_2
      (if (CallFunction|PawnAttackCheck _array_element_3)
        (Utilities|Array|Add (LocalVariables|GetAttack%20Array) _array_element_3))))
  (return (CallFunction|CleanPositionArray (LocalVariables|GetMovement%20Array)) (CallFunction|CleanPositionArray (LocalVariables|GetAttack%20Array))))