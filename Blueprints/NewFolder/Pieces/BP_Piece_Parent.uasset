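; Base chess piece actor that holds team, board position and selection state, with an empty move query as a hook for child pieces.
; Clicking a current-team piece highlights it through a dynamic material and sends its moves and attacks to the board.
; MovePiece updates the board's piece map, destroys any occupant, slides via timeline and signals completion.
; FindValidPath walks a direction, stopping before allies or on the first enemy.
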(event Custom|On%20Mouse%20Clicked
  (Variables|Default|SetIs%20Selected false))

(event Custom|MovePiece
  (params (Tile :type Primitive%20Component%20Object%20Reference))
  (bind _self self)
  (bind _board_reference (Variables|Default|GetBoard%20Reference))
  (bind _board_reference_2 (Variables|Default|GetBoard%20Reference))
  (bind _all_pieces_ (Variables|/Game/Blueprints/NewFolder/BP_ChessBoard.BP_ChessBoard_C|GetAll%20Pieces%20 _board_reference_2))
  (Utilities|Map|Remove (Variables|/Game/Blueprints/NewFolder/BP_ChessBoard.BP_ChessBoard_C|GetAll%20Pieces%20 _board_reference) (Variables|Default|GetPosition))
  (Variables|Default|SetHasMoved true)
  (bind _output_get (Variables|Default|SetPosition (Default|FindTileNumberandLetter _board_reference Tile)))
  (if (.Piece%20Found (Default|GetPositionInfo _board_reference _output_get))
    (Utilities|IsValid (.Piece (Default|GetPositionInfo _board_reference _output_get))
      (:Is%20Valid
        (Actor|DestroyActor (.Piece (Default|GetPositionInfo _board_reference _output_get)))
        (Utilities|Map|Remove _all_pieces_ _output_get))
      (:Is%20Not%20Valid
        _)))
  (Utilities|Map|Add _all_pieces_ _output_get self)
  (bind _newtrack_0 (Timeline|Movement%20Timeline PlayFromStart)
    (:Update
      (Transformation|SetActorLocation _self (Math|Vector|Lerp(Vector) (Transformation|GetWorldLocation Tile) (Transformation|GetActorLocation _self) _newtrack_0) false false))
    (:Finished
      (Default|CallPieceMoved (Variables|Default|GetTeam)))))

(event EventBeginPlay
  (bind _aschess_pc (Utilities|Casting|CastToChessPC (Game|GetPlayerController 0)))
  (EventDispatchers|BindEventtoMouseClicked _aschess_pc (delegate Custom|On%20Mouse%20Clicked))
  ;[1 1 1] Dynamic Material Ref
  (bind _returnvalue (Rendering|Material|CreateDynamicMaterialInstance (Variables|Default|GetStaticMesh) 0 "/Game/Chess_Assets/LightWoodMat_Parent.LightWoodMat_Parent" "None" :!class /Script/Engine.PrimitiveComponent))
  (Variables|Default|SetDynamic%20Material%20Ref _returnvalue))

(event MouseInput|EventActorOnClicked
  (params (ButtonPressed :type Key%20Structure :default "None"))
  (bind _board_reference (Variables|Default|GetBoard%20Reference))
  (if (Utilities|Enum|Equal(Enum) (Default|GetCurentTeam (Variables|Default|GetBoard%20Reference)) (Variables|Default|GetTeam))
    (Utilities|FlowControl|Delay 0.2)
    (Variables|Default|SetIs%20Selected true)
    (bind (_movement _attacks) (CallFunction|GetAllPossibleMoves))
    (Utilities|IsValid _board_reference
      (:Is%20Valid
        (Default|OnPieceSelected _board_reference self (CallFunction|CombineStringArray _movement _attacks))))))

(fn ConstructionScript)

(fn Init
  (params (Team :type TeamEnum%20Enum :default "NewEnumerator0") (Position :type String) (Board%20Reference :type BP%20Chess%20Board%20Object%20Reference))
  (bind _dynamic_material_ref (Variables|Default|GetDynamic%20Material%20Ref))
  (bind _output_get (Variables|Default|SetTeam Team))
  (Variables|Default|SetPosition Position)
  (Variables|Default|SetBoard%20Reference Board%20Reference)
  (Utilities|IsValid _dynamic_material_ref
    (:Is%20Valid
      (Rendering|Material|SetTextureParameterValue _dynamic_material_ref "TileTexture" (Utilities|Select :Index _output_get :NewEnumerator0 "/Game/Chess_Assets/LightWood.LightWood" :NewEnumerator1 "/Game/Chess_Assets/DarkWood1.DarkWood1")))))

(fn OnRepIsSelected
  (Rendering|Material|SetScalarParameterValue (Variables|Default|GetDynamic%20Material%20Ref) "Highlighted" (select (Variables|Default|GetIs%20Selected) 1.0 0.0) :!class /Script/Engine.MaterialInstanceDynamic))

(fn GetAllPossibleMoves
  (return 0 0))

(fn SetAllPossibleMoves
  (params (Current%20Movements :type Array%20of%20Strings) (Current%20Attacks :type Array%20of%20Strings))
  (Variables|Default|SetCurrent%20Movements Current%20Movements)
  (Variables|Default|SetCurrent%20Attacks Current%20Attacks))

(fn RefreshMoves
  (bind (_movement _attacks) (CallFunction|GetAllPossibleMoves))
  (CallFunction|SetAllPossibleMoves _movement _attacks))

(fn FindValidPath
  (params (Length :type Integer) (Direction :type DirectionEnum%20Enum :default "NewEnumerator0"))
  (bind _self self)
  (bind _local_array (LocalVariables|GetLocal%20Array))
  (bind _length (CallFunction|GetEdgeLength _self Direction))
  (bind _returnvalue (Math|Integer|Clamp(Integer) Length 0 _length))
  (if (> _returnvalue 0)
    (bind _index (Utilities|FlowControl|ForLoopwithBreak 1 _returnvalue :!label _label)
      (:LoopBody
        (if (.Piece%20Found (Default|GetPositionInfo (Variables|Default|GetBoard%20Reference) (CallFunction|GetPositioninDirection _index _self Direction)))
          (if (Utilities|Enum|Equal(Enum) (.Team (Default|GetPositionInfo (Variables|Default|GetBoard%20Reference) (CallFunction|GetPositioninDirection _index _self Direction))) (Variables|Default|GetTeam))
            (goto _label Break)
            (else
              (Utilities|Array|Add _local_array (CallFunction|GetPositioninDirection _index _self Direction))
              (goto _label Break)))
          (else
            (Utilities|Array|Add _local_array (CallFunction|GetPositioninDirection _index _self Direction)))))
      (:Completed
        (return (LocalVariables|GetLocal%20Array))))
    (else
      (return (LocalVariables|GetLocal%20Array)))))