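; BP_Knight is the chess knight piece, computing its candidate squares in GetAllPossibleMoves.
; It projects two squares in four directions, then offsets the letter by ±1 for two directions.
; The other two apply a zero number offset, yielding duplicate straight-line squares instead of L-shapes.
; BoardReference lookups blank same-team squares, and CleanPositionArray processes the identical Movement and Attacks lists.
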(event EventBeginPlay
  (|CallParentFunction) ; This node is disabled and will not be called.\nDrag off pins to build functionality.
)

(event Collision|EventActorBeginOverlap
  (params (OtherActor :type Actor%20Object%20Reference)))

(event EventTick
  (params (DeltaSeconds :type Float%20%28single-precision%29)))

(fn ConstructionScript
  (|CallParentFunction))

(fn GetAllPossibleMoves
  (bind _self self)
  (bind _self_2 self)
  (bind _self_3 self)
  (bind _self_4 self)
  (bind _board_reference (Variables|Default|GetBoard%20Reference))
  (bind _team (Variables|Default|GetTeam))
  (bind _board_reference_2 (Variables|Default|GetBoard%20Reference))
  (bind _team_2 (Variables|Default|GetTeam))
  (bind _board_reference_3 (Variables|Default|GetBoard%20Reference))
  (bind _team_3 (Variables|Default|GetTeam))
  (bind _board_reference_4 (Variables|Default|GetBoard%20Reference))
  (bind _team_4 (Variables|Default|GetTeam))
  (bind _position (CallFunction|GetPositioninDirection 2 _self "NewEnumerator1"))
  (bind _position_2 (CallFunction|GetPositioninDirection 2 _self_3 "NewEnumerator5"))
  (bind _position_3 (CallFunction|GetPositioninDirection 2 _self_4 "NewEnumerator0"))
  (bind _position_4 (CallFunction|GetPositioninDirection 2 _self_2 "NewEnumerator2"))
  (bind _output (CallFunction|GetPositionLetter _position))
  (bind _output_2 (CallFunction|GetPositionNumber _position_4))
  (bind _output_3 (CallFunction|GetPositionLetter _position_2))
  (bind _output_4 (CallFunction|GetPositionNumber _position_2))
  (bind _output_5 (CallFunction|GetPositionNumber _position))
  (bind _output_6 (CallFunction|GetPositionLetter _position_3))
  (bind _output_7 (CallFunction|GetPositionNumber _position_3))
  (bind _output_8 (CallFunction|GetPositionLetter _position_4))
  (bind _returnvalue (Math|Conversions|ToInteger(Byte) _output_2))
  (bind _return (CallFunction|GetNumberfromLetter _output))
  (bind _return_2 (CallFunction|GetNumberfromLetter _output_6))
  (bind _returnvalue_2 (Math|Conversions|ToInteger(Byte) _output_4))
  (bind _returnvalue_3 (Math|Conversions|ToInteger(Byte) _return))
  (bind _returnvalue_4 (Math|Conversions|ToInteger(Byte) _return_2))
  (bind _returnvalue_5 (+ _returnvalue_2 0))
  (bind _returnvalue_6 (- _returnvalue_2 0))
  (bind _returnvalue_7 (+ _returnvalue 0))
  (bind _returnvalue_8 (- _returnvalue 0))
  (bind _returnvalue_9 (Utilities|String|ToString(Integer) _returnvalue_7))
  (bind _returnvalue_10 (Utilities|String|ToString(Integer) _returnvalue_8))
  (bind _returnvalue_11 (Utilities|String|ToString(Integer) _returnvalue_6))
  (bind _returnvalue_12 (Utilities|String|ToString(Integer) _returnvalue_5))
  (bind _returnvalue_13 (+ _returnvalue_3 1))
  (bind _returnvalue_14 (- _returnvalue_3 1))
  (bind _returnvalue_15 (+ _returnvalue_4 1))
  (bind _returnvalue_16 (- _returnvalue_4 1))
  (bind _returnvalue_17 (Utilities|String|ToString(Integer) _returnvalue_14))
  (bind _returnvalue_18 (Utilities|String|ToString(Integer) _returnvalue_13))
  (bind _returnvalue_19 (Utilities|String|ToString(Integer) _returnvalue_15))
  (bind _returnvalue_20 (Utilities|String|ToString(Integer) _returnvalue_16))
  (bind _returnvalue_21 (Utilities|String|Append _output_3 _returnvalue_11))
  (bind _returnvalue_22 (Utilities|String|Append _output_3 _returnvalue_12))
  (bind _returnvalue_23 (Utilities|String|Append _output_8 _returnvalue_9))
  (bind _returnvalue_24 (Utilities|String|Append _output_8 _returnvalue_10))
  (bind (_piece _piece_found _team_5) (Default|GetPositionInfo _board_reference_2 _returnvalue_23))
  (bind (_piece_2 _piece_found_2 _team_6) (Default|GetPositionInfo _board_reference_2 _returnvalue_24))
  (bind _return_3 (CallFunction|GetLetterfromNumber _returnvalue_17))
  (bind _return_4 (CallFunction|GetLetterfromNumber _returnvalue_18))
  (bind (_piece_3 _piece_found_3 _team_7) (Default|GetPositionInfo _board_reference_3 _returnvalue_22))
  (bind (_piece_4 _piece_found_4 _team_8) (Default|GetPositionInfo _board_reference_3 _returnvalue_21))
  (bind _return_5 (CallFunction|GetLetterfromNumber _returnvalue_19))
  (bind _return_6 (CallFunction|GetLetterfromNumber _returnvalue_20))
  (bind _returnvalue_25 (Utilities|String|Append _return_5 _output_7))
  (bind _returnvalue_26 (Utilities|String|Append _return_6 _output_7))
  (bind _returnvalue_27 (Utilities|String|Append _return_3 _output_5))
  (bind _returnvalue_28 (Utilities|String|Append _return_4 _output_5))
  (bind _returnvalue_29 (Utilities|Enum|Equal(Enum) _team_5 _team_2))
  (bind _returnvalue_30 (Utilities|Enum|Equal(Enum) _team_2 _team_6))
  (bind _returnvalue_31 (Utilities|Enum|Equal(Enum) _team_7 _team_3))
  (bind _returnvalue_32 (Utilities|Enum|Equal(Enum) _team_3 _team_8))
  (bind (_piece_5 _piece_found_5 _team_9) (Default|GetPositionInfo _board_reference _returnvalue_27))
  (bind (_piece_6 _piece_found_6 _team_10) (Default|GetPositionInfo _board_reference_4 _returnvalue_25))
  (bind (_piece_7 _piece_found_7 _team_11) (Default|GetPositionInfo _board_reference_4 _returnvalue_26))
  (bind (_piece_8 _piece_found_8 _team_12) (Default|GetPositionInfo _board_reference _returnvalue_28))
  (bind _returnvalue_33 (and _piece_found_3 _returnvalue_31))
  (bind _returnvalue_34 (and _piece_found_4 _returnvalue_32))
  (bind _returnvalue_35 (and _piece_found _returnvalue_29))
  (bind _returnvalue_36 (and _piece_found_2 _returnvalue_30))
  (bind _returnvalue_37 (Utilities|Enum|Equal(Enum) _team _team_9))
  (bind _returnvalue_38 (Utilities|Enum|Equal(Enum) _team_12 _team))
  (bind _returnvalue_39 (Utilities|Enum|Equal(Enum) _team_10 _team_4))
  (bind _returnvalue_40 (Utilities|Enum|Equal(Enum) _team_4 _team_11))
  (bind _returnvalue_41 (select _returnvalue_35 "" _returnvalue_23))
  (bind _returnvalue_42 (select _returnvalue_36 "" _returnvalue_24))
  (bind _returnvalue_43 (select _returnvalue_33 "" _returnvalue_22))
  (bind _returnvalue_44 (select _returnvalue_34 "" _returnvalue_21))
  (bind _returnvalue_45 (and _piece_found_6 _returnvalue_39))
  (bind _returnvalue_46 (and _piece_found_7 _returnvalue_40))
  (bind _returnvalue_47 (and _piece_found_5 _returnvalue_37))
  (bind _returnvalue_48 (and _piece_found_8 _returnvalue_38))
  (bind _returnvalue_49 (select _returnvalue_47 "" _returnvalue_27))
  (bind _returnvalue_50 (select _returnvalue_48 "" _returnvalue_28))
  (bind _returnvalue_51 (select _returnvalue_45 "" _returnvalue_25))
  (bind _returnvalue_52 (select _returnvalue_46 "" _returnvalue_26))
  (bind _array (Utilities|Array|MakeArray _returnvalue_41 _returnvalue_42 _returnvalue_43 _returnvalue_44 _returnvalue_51 _returnvalue_52 _returnvalue_50 _returnvalue_49))
  (bind _return_array (CallFunction|CleanPositionArray _array))
  (return _return_array _return_array))