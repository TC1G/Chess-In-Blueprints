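; Chess king piece that generates its legal destinations, including castling to either side.
; GetAllPossibleMoves gathers one-square paths in all eight directions, adds castling squares, and returns the cleaned list as both movement and attacks.
; CanCastle requires an unmoved king not in check, an unmoved rook, and an empty, unthreatened path, with different distances per side.
; Valid castling destinations are cached in CastlinPoints, mapped to their direction.
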(event EventBeginPlay
  (|CallParentFunction) ; This node is disabled and will not be called.\nDrag off pins to build functionality.
)

(event Collision|EventActorBeginOverlap
  (params (OtherActor :type Actor%20Object%20Reference)))

(event EventTick
  (params (DeltaSeconds :type Float%20%28single-precision%29)))

(fn ConstructionScript
  (|CallParentFunction))

(fn GetAllPossibleMoves
  (Utilities|Map|Clear (Variables|Default|GetCastlinPoints))
  (for _array_element (Utilities|Array|MakeArray "NewEnumerator0" "NewEnumerator1" "NewEnumerator2" "NewEnumerator3" "NewEnumerator4" "NewEnumerator5" "NewEnumerator6" "NewEnumerator7")
    (bind _local_array1 (CallFunction|FindValidPath 1 _array_element))
    (LocalVariables|SetPoints (CallFunction|CombineStringArray _local_array1 (LocalVariables|GetPoints))))
  (if (CallFunction|CanCastle "NewEnumerator0")
    (Utilities|Map|Add (Variables|Default|GetCastlinPoints) (CallFunction|GetPositioninDirection 2 self "NewEnumerator0") "NewEnumerator0"))
  (if (CallFunction|CanCastle "NewEnumerator1")
    (Utilities|Map|Add (Variables|Default|GetCastlinPoints) (CallFunction|GetPositioninDirection 3 self "NewEnumerator1") "NewEnumerator1"))
  (bind _keys (Utilities|Map|Keys (Variables|Default|GetCastlinPoints)))
  (return (CallFunction|CleanPositionArray (CallFunction|CombineStringArray _keys (LocalVariables|GetPoints))) (CallFunction|CleanPositionArray (CallFunction|CombineStringArray _keys (LocalVariables|GetPoints)))))

(fn CanCastle
  (params (Direction :type DirectionEnum%20Enum :default "NewEnumerator0"))
  (bind _self self)
  (bind _self_2 self)
  (bind _board_reference (Variables|Default|GetBoard%20Reference))
  (bind _board_reference_2 (Variables|Default|GetBoard%20Reference))
  (bind _board_reference_3 (Variables|Default|GetBoard%20Reference))
  (bind _board_reference_4 (Variables|Default|GetBoard%20Reference))
  (bind _position (CallFunction|GetPositioninDirection 4 _self "NewEnumerator1"))
  (bind _position_2 (CallFunction|GetPositioninDirection 3 _self_2 "NewEnumerator0"))
  (bind (_piece _piece_found) (Default|GetPositionInfo _board_reference_3 _position))
  (bind (_piece_2 _piece_found_2) (Default|GetPositionInfo _board_reference_4 _position_2))
  (if (Default|IsKinginCheck (Variables|Default|GetBoard%20Reference))
    (return false)
    (elif (Variables|Default|GetHasMoved)
      (return false)
      (else
        (switch Utilities|FlowControl|Switch|SwitchonDirectionEnum Direction
          (:NewEnumerator0
            (if _piece_found_2
              (Utilities|IsValid _piece_2
                (:Is%20Valid
                  (if (== (Utilities|GetClass _piece_2) "/Game/Blueprints/NewFolder/Pieces/BP_Rook.BP_Rook_C")
                    (if (Variables|/Game/Blueprints/NewFolder/Pieces/BP_Piece_Parent.BP_Piece_Parent_C|GetHasMoved _piece_2)
                      (return false)
                      (else
                        (bind _local_array1 (CallFunction|FindValidPath 2 "NewEnumerator0"))
                        (if (> (Utilities|Array|Length _local_array1) 1)
                          (bind _array_element (Utilities|Array|ForEachLoopwithBreak _local_array1 :!label _label)
                            (:LoopBody
                              (if (.Piece%20Found (Default|GetPositionInfo _board_reference _array_element))
                                (LocalVariables|SetPathBroken true :!label _label_2)
                                (goto _label Break)
                                (elif (Default|IsPositioninDanger _board_reference _array_element (Variables|Default|GetTeam))
                                  (goto _label_2))))
                            (:Completed
                              (return (not (LocalVariables|GetPathBroken)))))
                          (else
                            (return false)))))
                    (else
                      (return false))))
                (:Is%20Not%20Valid
                  (return false)))
              (else
                (return false))))
          (:NewEnumerator1
            (if _piece_found
              (Utilities|IsValid _piece
                (:Is%20Valid
                  (if (== (Utilities|GetClass _piece) "/Game/Blueprints/NewFolder/Pieces/BP_Rook.BP_Rook_C")
                    (if (Variables|/Game/Blueprints/NewFolder/Pieces/BP_Piece_Parent.BP_Piece_Parent_C|GetHasMoved _piece)
                      (return false)
                      (else
                        (bind _local_array1_2 (CallFunction|FindValidPath 3 "NewEnumerator1"))
                        (if (> (Utilities|Array|Length _local_array1_2) 2)
                          (bind _array_element_2 (Utilities|Array|ForEachLoopwithBreak _local_array1_2 :!label _label_3)
                            (:LoopBody
                              (if (.Piece%20Found (Default|GetPositionInfo _board_reference_2 _array_element_2))
                                (LocalVariables|SetPathBroken true :!label _label_4)
                                (goto _label_3 Break)
                                (elif (Default|IsPositioninDanger _board_reference_2 _array_element_2 (Variables|Default|GetTeam))
                                  (goto _label_4))))
                            (:Completed
                              (return (not (LocalVariables|GetPathBroken)))))
                          (else
                            (return false)))))
                    (else
                      (return false))))
                (:Is%20Not%20Valid
                  (return false)))
              (else
                (return false)))))))))