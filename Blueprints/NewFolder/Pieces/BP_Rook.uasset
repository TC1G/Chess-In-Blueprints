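; BP_Rook is the rook piece Blueprint for a chess-style board game, supplying the squares it can move to or attack.
; Get All Possible Moves loops over four directions, using GetEdgeLength to bound each FindValidPath search toward the board edge.
; The paths are merged as string arrays, and the cleaned result is returned as both Movement and Attacks.
; NewFunction is empty and the event graph has no active logic.
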(event EventBeginPlay
  (|CallParentFunction) ; This node is disabled and will not be called.\nDrag off pins to build functionality.
)

(event Collision|EventActorBeginOverlap
  (params (OtherActor :type Actor%20Object%20Reference)))

(event EventTick
  (params (DeltaSeconds :type Float%20%28single-precision%29)))

(fn ConstructionScript
  (|CallParentFunction))

(fn NewFunction)

(fn GetAllPossibleMoves
  (for _array_element (Utilities|Array|MakeArray "NewEnumerator0" "NewEnumerator1" "NewEnumerator2" "NewEnumerator5")
    (bind _local_array1 (CallFunction|FindValidPath (CallFunction|GetEdgeLength self _array_element) _array_element))
    (LocalVariables|SetMS_Points (CallFunction|CombineStringArray _local_array1 (LocalVariables|GetMS_Points))))
  (return (CallFunction|CleanPositionArray (LocalVariables|GetMS_Points)) (CallFunction|CleanPositionArray (LocalVariables|GetMS_Points))))